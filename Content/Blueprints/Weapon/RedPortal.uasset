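; RedPortal is a portal actor that sends the MainCharacter to the blue portal when the character overlaps its Box.
; The destination location and rotation are read from BluePortalLoc and BluePortalRot stored on the character, with no direct reference to a blue portal actor.
; After moving the character, it sets player 0's control rotation and redirects velocity along the exit's forward vector at max movement speed, discarding entry momentum.
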(event `self.Box.OnComponentBeginOverlap`
  (params (OverlappedComponent :type "PrimitiveComponent Object Reference") (OtherActor :type "Actor Object Reference") (OtherComp :type "PrimitiveComponent Object Reference") (OtherBodyIndex :type Integer) (bFromSweep :type Boolean) (SweepResult :type "HitResult Structure (by ref)"))
  (bind _asmain_character (cast `/Game/Blueprints/Character/MainCharacter` OtherActor))
  (`self.K2_SetActorLocation` _asmain_character (`/Game/Blueprints/Character/MainCharacter.BluePortalLoc` _asmain_character) false false)
  (bind _blueportalrot (`/Game/Blueprints/Character/MainCharacter.BluePortalRot` _asmain_character))
  (`Controller.SetControlRotation` (`GameplayStatics.GetPlayerController` 0) _blueportalrot)
  (bind _charactermovement (`Character.CharacterMovement` _asmain_character))
  (set `MovementComponent.Velocity` (* (`KismetMathLibrary.GetForwardVector` _blueportalrot) (`MovementComponent.GetMaxSpeed` _charactermovement)) _charactermovement))

(fn `UserConstructionScript`)