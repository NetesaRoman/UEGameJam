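; Projectile for the blue portal gun shot that places a blue portal where it hits.
; On hit it ignores its instigator and destroys itself on actors tagged NoPortal.
; Otherwise it destroys any existing BluePortal, waiting briefly, then spawns a new one oriented to the hit normal.
; It stores the portal arrow's location and rotation on the player's MainCharacter, flags BluePlaced, and destroys itself.
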(event `self.ReceiveHit`
  (params (MyComp :type "PrimitiveComponent Object Reference") (Other :type "Actor Object Reference") (OtherComp :type "PrimitiveComponent Object Reference") (bSelfMoved :type Boolean) (HitLocation :type "Vector Structure") (HitNormal :type "Vector Structure") (NormalImpulse :type "Vector Structure") (Hit :type "HitResult Structure (by ref)"))
  (if (!= Other (`self.Instigator`))
    (if (`self.ActorHasTag` Other "NoPortal")
      (`self.K2_DestroyActor`)
      (else
        (`/Engine/EditorBlueprintResources/StandardMacros.IsValid` self
          (:`Is Valid`
            (bind _outactors (`GameplayStatics.GetAllActorsOfClass` "/Game/Blueprints/Weapon/BluePortal.BluePortal_C"))
            (bind _output (`|GetArrayItem` _outactors))
            (`/Engine/EditorBlueprintResources/StandardMacros.IsValid` _output
              (:`Is Valid`
                (`self.K2_DestroyActor` _output)
                (`KismetSystemLibrary.Delay` 0.1))
              (:`Is Not Valid`
                _))
            (bind _returnvalue (`|SpawnActorFromClass` "/Game/Blueprints/Weapon/BluePortal.BluePortal_C" (`KismetMathLibrary.MakeTransform` HitLocation (`KismetMathLibrary.MakeRotFromY` HitNormal)) "Undefined" "OverrideRootScale" null null))
            (bind _asmain_character (cast `/Game/Blueprints/Character/MainCharacter` (`GameplayStatics.GetPlayerCharacter` 0)))
            (bind _arrow (`/Game/Blueprints/Weapon/BluePortal.Arrow` _returnvalue))
            (set `/Game/Blueprints/Character/MainCharacter.BluePortalRot` (`KismetMathLibrary.Conv_VectorToRotator` (`SceneComponent.GetForwardVector` _arrow)) _asmain_character)
            (set `/Game/Blueprints/Character/MainCharacter.BluePortalLoc` (`SceneComponent.K2_GetComponentLocation` _arrow) _asmain_character)
            (set `/Game/Blueprints/Character/MainCharacter.BluePlaced` true _asmain_character)
            (`self.K2_DestroyActor`)))))))

(fn `UserConstructionScript`)