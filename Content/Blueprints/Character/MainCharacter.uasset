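; Player character Blueprint for a portal-shooting mechanic, with camera-relative movement, look and jump.
; Input axes move along the camera's forward and right vectors and turn the controller in pitch and yaw.
; Left and right mouse keys, bound directly, spawn blue and red portal projectiles respectively just ahead of the camera along its aim, each with a click sound at the spawn point.
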(event `InputAction|Jump`
  (params (Key :type "Key Structure"))
  ;[0.231 1 0.6818] Basic stuff
  (:`Pressed`
    (`self.Jump`))
  (:`Released`
    (`self.StopJumping`)))

(event `InputAxis|MoveForward`
  (params (AxisValue :type "Float (single-precision)"))
  ;[0.231 1 0.6818] Basic stuff
  (`self.AddMovementInput` (`SceneComponent.GetForwardVector` (`self.Camera`)) AxisValue))

(event `InputAxis|MoveRight`
  (params (AxisValue :type "Float (single-precision)"))
  ;[0.231 1 0.6818] Basic stuff
  (`self.AddMovementInput` (`SceneComponent.GetRightVector` (`self.Camera`)) AxisValue))

(event `InputAxis|LookUp`
  (params (AxisValue :type "Float (single-precision)"))
  ;[0.231 1 0.6818] Basic stuff
  (`self.AddControllerPitchInput` AxisValue))

(event `InputAxis|LookRight`
  (params (AxisValue :type "Float (single-precision)"))
  ;[0.231 1 0.6818] Basic stuff
  (`self.AddControllerYawInput` AxisValue))

(event `Key|LeftMouseButton`
  (params (Key :type "Key Structure"))
  (bind _returnvalue (`SceneComponent.K2_GetComponentRotation` (`self.Camera`)))
  (bind _returnvalue_2 (+ (+ (`SceneComponent.K2_GetComponentLocation` (`self.Camera`)) (`KismetMathLibrary.GreaterGreater_VectorRotator` (0.0 0.0 0.0) _returnvalue)) (* (`SceneComponent.GetForwardVector` (`self.Camera`)) 200.0)))
  (:`Pressed`
    (`|SpawnActorFromClass` "/Game/Blueprints/Weapon/BluePortal_Projectile.BluePortal_Projectile_C" (`KismetMathLibrary.MakeTransform` _returnvalue_2 _returnvalue) "Undefined" "OverrideRootScale" null null)
    (`GameplayStatics.PlaySoundAtLocation` "/Engine/VREditor/Sounds/UI/Click_on_Button.Click_on_Button" _returnvalue_2 (struct) 1.0 1.0 0.0 null null null null)))

(event `Key|RightMouseButton`
  (params (Key :type "Key Structure"))
  (bind _returnvalue (`SceneComponent.K2_GetComponentRotation` (`self.Camera`)))
  (bind _returnvalue_2 (+ (+ (`SceneComponent.K2_GetComponentLocation` (`self.Camera`)) (`KismetMathLibrary.GreaterGreater_VectorRotator` (0.0 0.0 0.0) _returnvalue)) (* (`SceneComponent.GetForwardVector` (`self.Camera`)) 200.0)))
  (:`Pressed`
    (`|SpawnActorFromClass` "/Game/Blueprints/Weapon/RedPortal_Projectile.RedPortal_Projectile_C" (`KismetMathLibrary.MakeTransform` _returnvalue_2 _returnvalue) "Undefined" "OverrideRootScale" null null)
    (`GameplayStatics.PlaySoundAtLocation` "/Engine/VREditor/Sounds/UI/Click_on_Button.Click_on_Button" _returnvalue_2 (struct) 1.0 1.0 0.0 null null null null)))

(fn `UserConstructionScript`)